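; Player controller Blueprint for a board game that sets up the game HUD and turns resolved clicks into unit selection and movement.
; On BeginPlay it sets the Action intent and fills the HUD with all BP_Player actors and the current hand.
; Clicking a unit selects it and sets Move intent.
; Board clicks convert to a tile for GridMovementComponent, clearing selection on success; the move checks for a selected unit, not the intent.
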(event `self.ReceiveBeginPlay`
  (bind _hudref (`self.HUDRef`))
  (`|ExecutionSequence`
    (:`then_0`
      (set `self.CurrentIntent` "Action"))
    (:`then_1`
      (bind _returnvalue (`|CreateWidget` "/Game/UI/WBP_GameHUD.WBP_GameHUD_C" self))
      (bind _output_get (set `self.HUDRef` _returnvalue))
      (`UserWidget.AddToViewport` _output_get 0)
      (bind _outactors (`GameplayStatics.GetAllActorsOfClass` "/Game/BPs/BP_Player.BP_Player_C"))
      (`/Game/UI/WBP_GameHUD.SetUnits` _hudref _outactors)
      (`/Game/UI/WBP_GameHUD.SetHand` _hudref (`self.GetCurrentHand`)))))

(event `self.BP_OnclickResolved`
  (params (Result :type "ClickResult Structure (by ref)"))
  (bind (_bhit _bhitunit _bhitboard _hitactor _worldpoint) (break `ClickResult` Result))
  ; Recibe el click de player y mira si hit on board o unit
  (`|ExecutionSequence`
    (:`then_0`
      ; Selección unit, lo guarda y entra en mode:Move
      (if _bhitunit
        (bind _asbp_unit (cast `/Game/BPs/Characters/BP_Unit` _hitactor))
        (set `self.selectedUnit` _asbp_unit)
        (set `self.CurrentIntent` "Move")
        (`KismetSystemLibrary.PrintString` "BLUEPRINT: Unidad seleccionada")))
    (:`then_1`
      ; Solo se mueve si: Click sobre board , hay unit seleccionada y esta en modo Move
      (if _bhitboard
        (`/Engine/EditorBlueprintResources/StandardMacros.IsValid` (`self.selectedUnit`)
          (:`Is Valid`
            ; Convierte el punto en casilla
            (bind _asbp_board (cast `/Game/BPs/Board/BP_Board` _hitactor))
            (bind (_outtile _returnvalue) (`Board.WorldPointToTile` _asbp_board _worldpoint))
            (if _returnvalue
              (bind _returnvalue_2 (`GridMovementComponent.moveToTile` (`self.GetComponentByClass` (`self.selectedUnit`) "/Script/Egnis.GridMovementComponent") _outtile)) ; Intenta mover casilla
              (if _returnvalue_2
                (set `self.selectedUnit` null) ; Por defecto none.LIMPIEZA
                (set `self.CurrentIntent` "Action")
                (`KismetSystemLibrary.PrintString` "BLUEPRINT: Movido")
                (else
                  (`KismetSystemLibrary.PrintString` "BLUEPRINT: No se ha movido")))
              (else
                (`KismetSystemLibrary.PrintString` "BLUEPRINT: No se pudo convertir el punto a  casilla")))))))))

(fn `UserConstructionScript`)